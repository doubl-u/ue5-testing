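; Base enemy character Blueprint that carries a weapon and provides attack, patrol route and movement speed functions.
; On BeginPlay or attachTheWeapon, it spawns a scaled-down BP_W2, snaps it to the mesh's weaponSocket and flags it as wielded.
; The default attack is a placeholder that prints, waits briefly, then fires the OnAtkExecuted dispatcher.
; Helper functions return the Route and map a speed state to MaxWalkSpeed.
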(event Custom|attack
  (Development|PrintString "defaultATK executed.")
  (Utilities|FlowControl|Delay 0.5)
  (Default|CallOnAtkExecuted))

(event Custom|attachTheWeapon
  (bind _returnvalue (Transformation|GetActorTransform))
  (Development|PrintString "weapon attached")
  (bind _returnvalue_2 (Game|SpawnActorfromClass "/Game/Weapon/BP_W2.BP_W2_C" (Math|Transform|MakeTransform (.location _returnvalue) (.rotation _returnvalue) "0.100000,0.100000,0.100000") "Undefined" "MultiplyWithRoot" 0 0))
  (Transformation|AttachComponentToComponent _returnvalue_2 (Variables|Character|GetMesh) "weaponSocket" "SnapToTarget" "SnapToTarget" "SnapToTarget" true)
  (Variables|Default|Setis%20weilding%20weapon true))

(event EventBeginPlay
  (bind _returnvalue (Transformation|GetActorTransform))
  (bind _returnvalue_2 (Game|SpawnActorfromClass "/Game/Weapon/BP_W2.BP_W2_C" (Math|Transform|MakeTransform (.location _returnvalue) (.rotation _returnvalue) "0.100000,0.100000,0.100000") "Undefined" "MultiplyWithRoot" 0 0))
  (Transformation|AttachComponentToComponent _returnvalue_2 (Variables|Character|GetMesh) "weaponSocket" "SnapToTarget" "SnapToTarget" "SnapToTarget" true)
  (Variables|Default|Setis%20weilding%20weapon true))

(fn ConstructionScript)

(fn GetPatrolRoute
  (return (Variables|Default|GetRoute)))

(fn SetMovementSpeed
  (params (speed :type movementSpeed%20Enum :default "NewEnumerator0"))
  (bind _output_get (Variables|/Script/Engine.CharacterMovementComponent|SetMaxWalkSpeed (Variables|Character|GetCharacterMovement) (Utilities|Select :Index speed :NewEnumerator0 0.0 :NewEnumerator1 1e+02 :NewEnumerator2 3e+02 :NewEnumerator3 5e+02)))
  (return _output_get))