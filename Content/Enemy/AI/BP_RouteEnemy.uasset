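; BP_RouteEnemy holds spline patrol route state for an enemy, tracking a point index and a direction.
; IncrementPatrolRoute always adds one to PatrolIndex, then sets Direction to -1 if the spline's point count equals -1, or to 1 if the index is 0.
; Direction never feeds back into the increment here.
; GetSplinePointWorldLoc returns the world location of the current spline point.
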(event Custom|IncrementPatrolRoute
  (bind _result (Math|Integer|IncrementInt (Variables|Default|GetPatrolIndex))
    (:%20%20
      (Variables|Default|SetPatrolIndex _result)
      (if (== (Spline|GetNumberOfSplinePoints (Variables|Default|GetpatrolRoute)) -1)
        (Variables|Default|SetDirection -1)
        (elif (== (Variables|Default|GetPatrolIndex) 0)
          (Variables|Default|SetDirection 1))))))

(fn ConstructionScript)

(fn GetSplinePointWorldLoc
  (return (Spline|GetLocationatSplinePoint (Variables|Default|GetpatrolRoute) (Variables|Default|GetPatrolIndex) "World")))